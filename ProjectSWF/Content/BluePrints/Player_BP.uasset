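; Player character Blueprint that handles basic attack and dash input, with dashing along the world X axis.
; Basic attack raises an Attacking flag for a short timed window.
; Dash sets a fixed X velocity in the direction of movement, falling back to control yaw when there is no X movement.
; It briefly zeroes gravity and ground friction, then restores them, with a DoOnce reset after a delay acting as cooldown.
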(event Input|ActionEvents|InputActionBasicAttack
  (params (Key :type Key%20Structure :default "None"))
  (:Pressed
    (Variables|Default|SetAttacking true)
    (Utilities|FlowControl|Delay 0.46)
    (Variables|Default|SetAttacking false)))

(event Input|ActionEvents|InputActionDash
  (params (Key :type Key%20Structure :default "None"))
  (bind _charactermovement (Variables|Character|GetCharacterMovement))
  (bind _returnvalue (Pawn|Components|CharacterMovement|GetLastUpdateVelocity _charactermovement))
  (:Pressed
    (Utilities|FlowControl|DoOnce false :!label _label
      (:Completed
        (if (> (.x _returnvalue) 0.0)
          (Variables|/Script/Engine.MovementComponent|SetVelocity _charactermovement "3000.000000, 0, 0" :!label _label_2)
          (else
            (if (> 0.0 (.x _returnvalue))
              _
              (elif (> (.yaw (Pawn|GetControlRotation :!class /Script/Engine.Pawn)) 9e+01)
                _
                (else
                  (goto _label_2))))
            (Variables|/Script/Engine.MovementComponent|SetVelocity _charactermovement "-3000.000000, 0, 0")))
        (Variables|/Script/Engine.CharacterMovementComponent|SetGravityScale _charactermovement 0.0)
        (Variables|/Script/Engine.CharacterMovementComponent|SetGroundFriction _charactermovement 0.0)
        (Utilities|FlowControl|Delay 0.23)
        (Variables|/Script/Engine.CharacterMovementComponent|SetGravityScale _charactermovement 4.0)
        (Variables|/Script/Engine.CharacterMovementComponent|SetGroundFriction _charactermovement 5e+01)
        (Utilities|FlowControl|Delay 0.4)
        (goto _label Reset)))))

(fn ConstructionScript)