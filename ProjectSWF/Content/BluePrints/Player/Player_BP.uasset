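; Player Blueprint that handles the basic attack and a horizontal dodge along the X axis.
; Attack input passes a DoOnce gate to spawn a hitbox and briefly set Attacking.
; Dodge clears Attacking, disables input and launches along velocity direction, or control yaw when still, suspending gravity and ground friction for its duration.
; Airborne dodges consume NumDodge, which is not replenished in this graph, while grounded dodges bypass that check.
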(event Input|ActionEvents|InputActionBasicAttack
  (params (Key :type Key%20Structure :default "None"))
  ;[1 1 1] BasicAttack Detect    // TODO be careful of dodging (may need to check Dodging status first)
  (:Pressed
    (Utilities|FlowControl|DoOnce false :!label _label
      (:Completed
        (Class|ProjectSWFCharacter|SpawnHitBox)
        (Variables|Default|SetAttacking true)
        (Utilities|FlowControl|Delay 0.33)
        (Variables|Default|SetAttacking false)
        (goto _label Reset)))))

(event Input|ActionEvents|InputActionDodge
  (params (Key :type Key%20Structure :default "None"))
  (bind _charactermovement (Variables|Character|GetCharacterMovement))
  (bind _returnvalue (Pawn|Components|CharacterMovement|GetLastUpdateVelocity _charactermovement))
  ;[1 1 1] Dodging
  (:Pressed
    (if (not (Variables|Default|GetDodging))
      (if (AI|Components|NavMovement|IsFalling (Variables|Character|GetCharacterMovement))
        (if (== (Variables|Default|GetNumDodge) 1)
          (Variables|Default|SetNumDodge 0)
          (Variables|Default|SetAttacking false :!label _label)
          (Variables|Default|SetDodging true)
          (Input|DisableInput 0)
          (if (> (.x _returnvalue) 0.0)
            (Variables|/Script/Engine.MovementComponent|SetVelocity _charactermovement "2000.000000, 0, 0" :!label _label_2)
            (else
              (if (> 0.0 (.x _returnvalue))
                _
                (elif (> (.yaw (Pawn|GetControlRotation :!class /Script/Engine.Pawn)) 9e+01)
                  _
                  (else
                    (goto _label_2))))
              (Variables|/Script/Engine.MovementComponent|SetVelocity _charactermovement "-2000.000000, 0, 0")))
          (Variables|/Script/Engine.CharacterMovementComponent|SetGravityScale _charactermovement 0.0)
          (Variables|/Script/Engine.CharacterMovementComponent|SetGroundFriction _charactermovement 0.0)
          (Utilities|FlowControl|Delay 0.5)
          (Variables|/Script/Engine.CharacterMovementComponent|SetGravityScale _charactermovement 4.0)
          (Variables|/Script/Engine.CharacterMovementComponent|SetGroundFriction _charactermovement 5e+01)
          (Input|EnableInput 0)
          (Variables|Default|SetDodging false)
          (Utilities|FlowControl|Delay 0.1))
        (else
          (goto _label))))))

(fn ConstructionScript)