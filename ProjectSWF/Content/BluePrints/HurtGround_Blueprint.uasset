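; Hurting ground hazard that damages, slows and tints the 2D player character (Player_BP) standing on it.
; On actor overlap it colors the sprite orange-red, applies the hurt walk speed and deals 1 damage with debug text.
; A one-second Delay loop repeats the damage while the player's capsule overlaps HitBox.
; Any HitBox end overlap restores normal speed on the cached player, then resets the tint after a short delay.
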(event OnComponentEndOverlap(HitBox)
  (params (OverlappedComponent :type Primitive%20Component%20Object%20Reference) (OtherActor :type Actor%20Object%20Reference) (OtherComp :type Primitive%20Component%20Object%20Reference) (OtherBodyIndex :type Integer))
  ;[1 1 1] Hurting Ground
  (Variables|/Script/Engine.CharacterMovementComponent|SetMaxWalkSpeed (Variables|/Script/Engine.Character|GetCharacterMovement (stale Collision|EventActorBeginOverlap _asplayer_bp)) (Variables|/Game/BluePrints/Player/Player_BP.Player_BP_C|GetNormalMaxWalkSpeed (stale Collision|EventActorBeginOverlap _asplayer_bp)))
  (Utilities|FlowControl|Delay 0.3)
  (Sprite|SetSpriteColor (Variables|/Script/Paper2D.PaperCharacter|GetSprite (stale Collision|EventActorBeginOverlap _asplayer_bp)) "(R=1.000000,G=1.000000,B=1.000000,A=1.000000)"))

(event EventBeginPlay)

(event Collision|EventActorBeginOverlap
  (params (OtherActor :type Actor%20Object%20Reference))
  ;[1 1 1] Hurting Ground
  (bind _asplayer_bp (Utilities|Casting|CastToPlayer_BP OtherActor))
  (Sprite|SetSpriteColor (Variables|/Script/Paper2D.PaperCharacter|GetSprite _asplayer_bp) "(R=1.000000,G=0.238338,B=0.000000,A=0.661000)")
  (Variables|/Script/Engine.CharacterMovementComponent|SetMaxWalkSpeed (Variables|/Script/Engine.Character|GetCharacterMovement _asplayer_bp) (Variables|/Game/BluePrints/Player/Player_BP.Player_BP_C|GetHurtWalkSpeed _asplayer_bp))
  (Class|ProjectSWFCharacter|TakeDamage _asplayer_bp 1 :!label _label)
  (Development|PrintText "-1 hp")
  (Utilities|FlowControl|Delay 1.0)
  (if (Class|PrimitiveComponent|IsOverlappingComponent (Variables|/Script/Engine.Character|GetCapsuleComponent _asplayer_bp) (Variables|Default|GetHit%20Box))
    (goto _label)))

(event EventTick
  (params (DeltaSeconds :type Float%20%28single-precision%29)))

(fn ConstructionScript)