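; Enemy Blueprint that patrols along walk paths and pursues the player when detected.
; BeginPlay attaches its Status, and while no player is spotted, capsule overlaps with a WalkPath_BP make it halt and reverse direction.
; A Detection overlap volume starts walking towards a Player_BP on entry and calls the lose-track logic when the player leaves.
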(event OnComponentBeginOverlap(CapsuleComponent)
  (params (OverlappedComponent :type Primitive%20Component%20Object%20Reference) (OtherActor :type Actor%20Object%20Reference) (OtherComp :type Primitive%20Component%20Object%20Reference) (OtherBodyIndex :type Integer) (bFromSweep :type Boolean) (SweepResult :type Hit%20Result%20Structure%20%28by%20ref%29))
  ;[1 1 1] Normal Parade and Halt
  (bind _returnvalue (Class|Enemy02|ReturnPlayerSpotted))
  (if (not _returnvalue)
    (Utilities|Casting|CastToWalkPath_BP OtherActor)
    (Class|Enemy02|MakeHalt)
    (Class|Enemy02|ReverseDirection)))

(event OnComponentBeginOverlap(Detection)
  (params (OverlappedComponent :type Primitive%20Component%20Object%20Reference) (OtherActor :type Actor%20Object%20Reference) (OtherComp :type Primitive%20Component%20Object%20Reference) (OtherBodyIndex :type Integer) (bFromSweep :type Boolean) (SweepResult :type Hit%20Result%20Structure%20%28by%20ref%29))
  ;[1 1 1] Walk Towards Player when spotted
  (Utilities|Casting|CastToPlayer_BP OtherActor)
  (Class|Enemy02|WalkTowardsPlayer))

(event OnComponentEndOverlap(Detection)
  (params (OverlappedComponent :type Primitive%20Component%20Object%20Reference) (OtherActor :type Actor%20Object%20Reference) (OtherComp :type Primitive%20Component%20Object%20Reference) (OtherBodyIndex :type Integer))
  ;[1 1 1] Action when lose track of player
  (Utilities|Casting|CastToPlayer_BP OtherActor)
  (Class|Enemy02|LoseTrackOfPlayer))

(event EventBeginPlay
  ;[1 1 1] Setup
  (Class|Enemy02|AttachStatus (Variables|Default|GetStatus)))

(fn ConstructionScript)