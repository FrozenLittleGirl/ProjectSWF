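; Hitbox actor for Enemy03's basic attack that damages and pushes the player during a short active window.
; On BeginPlay it attaches its HitBox, then destroys itself after PersistTime, which matches the hit duration.
; Overlaps with Player_BP's capsule apply damage and force along the direction from ReturnDirection.
; Overlaps with Enemy-tagged actors call IgnoreActorWhenMoving on Body, with no actor specified.
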(event OnComponentBeginOverlap(HitBox)
  (params (OverlappedComponent :type Primitive%20Component%20Object%20Reference) (OtherActor :type Actor%20Object%20Reference) (OtherComp :type Primitive%20Component%20Object%20Reference) (OtherBodyIndex :type Integer) (bFromSweep :type Boolean) (SweepResult :type Hit%20Result%20Structure%20%28by%20ref%29))
  (if (Actor|ActorHasTag OtherActor "Enemy")
    (Collision|IgnoreActorwhenMoving (Variables|Default|GetBody) 0 true))
  (bind _asplayer_bp (Utilities|Casting|CastToPlayer_BP OtherActor))
  (if (== (Variables|/Script/Engine.Character|GetCapsuleComponent _asplayer_bp) OtherComp)
    (bind _returnvalue (Class|HitBoxActor|ReturnDirection))
    (Class|ProjectSWFCharacter|TakeDamage _asplayer_bp (Variables|Default|GetDamage) _returnvalue (Variables|Default|GetForce))))

(event EventBeginPlay
  ;[1 1 1] Basic Attack (delay is same as hitting time)
  (Class|HitBoxActor|AttachHitBox (Variables|Default|GetHitBox))
  (Utilities|FlowControl|Delay (Variables|Default|GetPersistTime))
  (Actor|DestroyActor))

(fn ConstructionScript)